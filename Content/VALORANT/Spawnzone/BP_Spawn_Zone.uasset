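; BP_Spawn_Zone is a spawn area that keeps an enemy in play, creating a BP_Enemy at BeginPlay and another after a death.
; Each spawn takes a random X and Y inside BoxSpawnZone, with Z set to the box's bottom plus an offset to sit on the ground.
; The new enemy's OnDeath is bound to OnEnemyDeath, which increments NumberRounds and spawns again unless that count equals zero.
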(event Custom|Spawn_Enemy
  (bind _box_spawn_zone (Variables|Default|GetBox_Spawn_Zone))
  (bind _returnvalue (Transformation|GetWorldLocation _box_spawn_zone))
  (bind _returnvalue_2 (Components|Box|GetScaledBoxExtent _box_spawn_zone))
  (bind _returnvalue_3 (Math|Random|RandomPointinBoundingBox _returnvalue _returnvalue_2))
  (bind (_x _y) (Math|Vector|BreakVector _returnvalue_3))
  (bind _returnvalue_4 (Game|SpawnActorfromClass "/Game/VALORANT/Spawnzone/BP_Enemy.BP_Enemy_C" (Math|Transform|MakeTransform (Math|Vector|MakeVector _x _y (+ (- (.Z (Math|Vector|BreakVector _returnvalue)) (.Z (Math|Vector|BreakVector _returnvalue_2))) (Variables|Default|GetOffset)))) "Undefined" "MultiplyWithRoot" 0 0))
  (EventDispatchers|BindEventtoOnDeath _returnvalue_4 (delegate Custom|On%20Enemy%20Death)))

(event Custom|On%20Enemy%20Death
  (Utilities|FlowControl|Sequence
    (:then_0
      (Variables|Default|SetNumber_Rounds (+ (Variables|Default|GetNumber_Rounds) 1)))
    (:then_1
      (if (== (Variables|Default|GetNumber_Rounds) 0)
        (Variables|Default|SetNumber_Rounds (+ (Variables|Default|GetNumber_Rounds) 1))
        (else
          (CallFunction|SpawnEnemy))))))

(event EventBeginPlay
  (CallFunction|SpawnEnemy))

(fn ConstructionScript)