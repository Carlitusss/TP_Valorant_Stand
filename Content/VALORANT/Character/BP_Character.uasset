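; BP_Character is a player character Blueprint for a Valorant-style first-person game, handling Enhanced Input movement.
; On BeginPlay it casts the controller to BP_FirstPersonPlayerController and adds the IMC_Valorant mapping context.
; Forward/back and right/left input actions call AddMovementInput along directions derived from control rotation, with pitch zeroed so looking up or down leaves movement direction unaffected.
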(event Input|EnhancedActionEvents|EnhancedInputActionIA_Move_Fwd_Bwd
  (params (ActionValue :type Float%20%28double-precision%29) (ElapsedSeconds :type Float%20%28double-precision%29) (TriggeredSeconds :type Float%20%28double-precision%29) (InputAction :type Input%20Action%20Object%20Reference :default "/Game/VALORANT/Character/Actions/IA_Move_Fwd_Bwd.IA_Move_Fwd_Bwd"))
  ;[0 0 0] Add Movement Input
  ;;[1 1 1] Move Fwd / Bwd
  (:Triggered
    (Pawn|Input|AddMovementInput (Math|Vector|GetForwardVector (Math|Rotator|MakeRotator 0.0 0.0 (.Yaw (Math|Rotator|BreakRotator (Pawn|GetControlRotation (Game|GetPlayerController 0) :!class /Script/Engine.Controller))))) ActionValue false)))

(event Input|EnhancedActionEvents|EnhancedInputActionIA_Move_Right_Left
  (params (ActionValue :type Float%20%28double-precision%29) (ElapsedSeconds :type Float%20%28double-precision%29) (TriggeredSeconds :type Float%20%28double-precision%29) (InputAction :type Input%20Action%20Object%20Reference :default "/Game/VALORANT/Character/Actions/IA_Move_Right_Left.IA_Move_Right_Left"))
  (bind _returnvalue (Game|GetPlayerController 0))
  (bind _returnvalue_2 (Pawn|GetControlRotation _returnvalue :!class /Script/Engine.Controller))
  (bind (_roll _pitch _yaw) (Math|Rotator|BreakRotator _returnvalue_2))
  ;[0 0 0] Add Movement Input
  ;;[1 1 1] Move Right / Left
  (:Triggered
    (Pawn|Input|AddMovementInput (Math|Vector|GetRightVector (Math|Rotator|MakeRotator _roll 0.0 _yaw)) ActionValue false)))

(event EventBeginPlay
  ;[0 0 0] Add Mapping Context
  (bind _asbp_first_person_player_controller (Utilities|Casting|CastToBP_FirstPersonPlayerController (Game|GetPlayerController 0)))
  (Utilities|IsValid (PlayerController|LocalPlayerSubsystems|GetEnhancedInputLocalPlayerSubsystem _asbp_first_person_player_controller)
    (:Is%20Valid
      (Input|AddMappingContext (PlayerController|LocalPlayerSubsystems|GetEnhancedInputLocalPlayerSubsystem _asbp_first_person_player_controller) "/Game/VALORANT/Character/Actions/IMC/IMC_Valorant.IMC_Valorant" 0 "(bIgnoreAllPressedKeysUntilRelease=True,bForceImmediately=False,bNotifyUserSettings=False)"))))

(fn ConstructionScript)